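; Toon Tanks game mode that handles game start and end, treating levels containing a GM_MenuActor as menus.
; In menu levels, the construction script selects BP_StartPawnTank as default pawn, and StartGame shows the menu widget, disables tank input and enables the cursor.
; Other levels get the game-start widget.
; GameOver shows the result, then after a delay reloads on loss or sets Level1Passed in BP_GI and opens Main on win.
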(event EventStartGame
  (bind _outactors (Actor|GetAllActorsOfClass "/Game/Blueprints/Gamemodes/GM_MenuActor.GM_MenuActor_C"))
  (if (Utilities|Array|IsEmpty _outactors)
    (bind _returnvalue (UserInterface|CreateWidget "/Game/Blueprints/Widgets/WBP_GameStart.WBP_GameStart_C"))
    (UserInterface|Viewport|AddtoViewport _returnvalue 0)
    (else
      (bind _returnvalue_2 (UserInterface|CreateWidget "/Game/Blueprints/Widgets/WBP_StartGame.WBP_StartGame_C"))
      (UserInterface|Viewport|AddtoViewport _returnvalue_2 0)
      (bind _outactors_2 (Actor|GetAllActorsOfClass "/Game/Blueprints/Pawns/BP_StartPawnTank.BP_StartPawnTank_C"))
      (bind _asplayer_controller (Utilities|Casting|CastToPlayerController (Pawn|GetController (Utilities|Array|Get(acopy) _outactors_2))))
      (Input|DisableInput (Utilities|Array|Get(acopy) _outactors_2) _asplayer_controller)
      (Variables|/Script/Engine.PlayerController|SetbShowMouseCursor _asplayer_controller true)
      (Variables|/Script/Engine.PlayerController|SetCurrentMouseCursor (Game|GetPlayerController 0) "Default"))))

(event EventGameOver
  (params (bGameOverCond :type Boolean))
  (bind _returnvalue (UserInterface|CreateWidget "/Game/Blueprints/Widgets/WBP_EndGame.WBP_EndGame_C"))
  (Rendering|Components|TextRender|SetText (Variables|/Game/Blueprints/Widgets/WBP_EndGame.WBP_EndGame_C|GetDisplayText _returnvalue) (select bGameOverCond "You Lost!" "You Won!"))
  (UserInterface|Viewport|AddtoViewport _returnvalue 0)
  (if bGameOverCond
    (Utilities|FlowControl|Delay 3.0)
    (bind _returnvalue_2 (Game|GetCurrentLevelName true))
    (Game|OpenLevel(byName) (Utilities|String|StringToName _returnvalue_2))
    (else
      (Utilities|FlowControl|Delay 5.0)
      (bind _asbp_gi (Utilities|Casting|CastToBP_GI (Game|GetGameInstance)))
      (Variables|/Game/Blueprints/BP_GI.BP_GI_C|SetLevel1Passed? _asbp_gi true)
      (Game|OpenLevel(byObjectReference) "/Game/Maps/Main.Main"))))

(fn ConstructionScript
  (bind _outactors (Actor|GetAllActorsOfClass "/Game/Blueprints/Gamemodes/GM_MenuActor.GM_MenuActor_C"))
  (if (not (Utilities|Array|IsEmpty _outactors))
    (Variables|Default|SetDefaultPawnClass "/Game/Blueprints/Pawns/BP_StartPawnTank.BP_StartPawnTank_C")))